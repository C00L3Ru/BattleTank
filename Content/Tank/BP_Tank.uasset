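; Tank pawn that the player drives, aims and fires through input bindings.
; Construction and BeginPlay register the turret and barrel references, and BeginPlay also initialises the movement component with both tracks.
; Aim axes rotate an azimuth gimbal for yaw and a spring arm for pitch, keeping the two rotations separate.
; Per-track throttle axes drive each track directly, while MoveForward passes intent to the movement component.
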(event `self.ReceiveBeginPlay`
  (`self.SetTurretReference` (`self.TankTurret`))
  (`self.SetBarrelReference` (`self.TankBarrel`))
  (`TankMovementComponent.Initialise` (`self.TankMovement`) (`self.TankTrackL`) (`self.TankTrackR`)))

(event `InputAxis|AimAzimuth`
  (params (AxisValue :type "Float (single-precision)"))
  (`SceneComponent.K2_AddLocalRotation` (`self.AzimuthGimbal`) (`KismetMathLibrary.MakeRotator` 0.0 0.0 AxisValue) false false))

(event `InputAxis|AimElevation`
  (params (AxisValue :type "Float (single-precision)"))
  (`SceneComponent.K2_AddLocalRotation` (`self.SpringArm1`) (`KismetMathLibrary.MakeRotator` 0.0 AxisValue) false false))

(event `InputAction|Fire`
  (params (Key :type "Key Structure"))
  (:`Pressed`
    (`self.Fire`)))

(event `InputAxis|LeftThrottle`
  (params (AxisValue :type "Float (single-precision)"))
  (`TankTrack.SetThrottle` (`self.TankTrackL`) AxisValue))

(event `InputAxis|RightThrottle`
  (params (AxisValue :type "Float (single-precision)"))
  (`TankTrack.SetThrottle` (`self.TankTrackR`) AxisValue))

(event `InputAxis|MoveForward`
  (params (AxisValue :type "Float (single-precision)"))
  (`TankMovementComponent.IntendMoveForward` (`self.TankMovement`) AxisValue))

(fn `UserConstructionScript`
  (`self.SetTurretReference` (`self.TankTurret`))
  (`self.SetBarrelReference` (`self.TankBarrel`)))